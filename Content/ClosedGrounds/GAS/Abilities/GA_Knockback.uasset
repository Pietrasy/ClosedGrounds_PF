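; GA_Knockback is a Gameplay Ability that shoves its avatar backward, opposite its forward vector.
; On successful commit, an Apply Root Motion Constant Force task applies a short burst, then sets velocity from the avatar's current velocity.
; A failed commit prints a debug message and ends the ability.
; The success path never calls End Ability, as that node is disconnected; ending only prints a debug message.
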(event `self.K2_ActivateAbility`
  (bind _returnvalue (`self.GetAvatarActorFromActorInfo`))
  (`parent.K2_ActivateAbility`)
  (bind _returnvalue_2 (`self.K2_CommitAbility`))
  (if _returnvalue_2
    (`AbilityTask_ApplyRootMotionConstantForce.ApplyRootMotionConstantForce` "None" (`KismetMathLibrary.NegateVector` (`Actor.GetActorForwardVector` _returnvalue)) 2000.0 0.2 false null "SetVelocity" (`Actor.GetVelocity` _returnvalue))
    (else
      (`KismetSystemLibrary.PrintString` "Ability false")
      (`self.K2_EndAbility`))))

(event `self.K2_OnEndAbility`
  (params (bWasCancelled :type Boolean))
  (`KismetSystemLibrary.PrintString` "Knockback finished"))