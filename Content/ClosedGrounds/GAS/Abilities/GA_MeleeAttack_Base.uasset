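; Base melee attack Gameplay Ability that arms the avatar's weapons with a damage effect and plays an attack montage.
; On activation it commits, caches the avatar's CG_WeaponComponent, and gives every weapon an effect spec carrying a set-by-caller damage magnitude.
; It then plays the montage, exposing an empty MontageStarted event, and ends when the montage completes, is interrupted or is cancelled.
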(event `self.K2_ActivateAbility`
  (bind _returnvalue (`self.K2_CommitAbility`))
  (if _returnvalue
    (`self.CacheWeaponComponent`)
    (for _array_element (`CG_WeaponComponent.Weapons` (`self.WeaponComponent`))
      (`self.AddEffectToWeapon` _array_element))
    (`self.OnMontageStart`)
    (else
      (`KismetSystemLibrary.PrintString` "Ability wasn't commited!")
      (`self.K2_EndAbility`))))

(event `OnMontageStart`
  (`self.AttackMontage`
    (:`then`
      (`AbilityTask_PlayMontageAndWait.CreatePlayMontageAndWaitProxy` "None" (`self.AttackMontage`)
        (:`then`
          (`self.MontageStarted`))
        (:`OnCompleted`
          (`self.K2_EndAbility` :!label _label))
        (:`OnInterrupted`
          (goto _label))
        (:`OnCancelled`
          (goto _label))))
    (:`else`
      (`self.K2_EndAbility`))))

(event `MontageStarted`)

(fn `AddEffectToWeapon`
  (params (Weapon :type "CG_Weapon Object Reference"))
  (`/Engine/EditorBlueprintResources/StandardMacros.IsValid` Weapon
    (:`Is Valid`
      (bind _returnvalue (`AbilitySystemBlueprintLibrary.AssignTagSetByCallerMagnitude` (`self.MakeOutgoingGameplayEffectSpec` (`self.EffectClass`)) (struct :`TagName` "GAS.Data.Damage") (`self.DamageMagnitude`)))
      (`CG_Weapon.SetEffectToWeapon` (`local.Weapon`) _returnvalue)
      (return))
    (:`Is Not Valid`
      (`KismetSystemLibrary.PrintString` "CurrentWeapon isn't valid!"))))

(fn `CacheWeaponComponent`
  (bind _returnvalue (`Actor.GetComponentByClass` (`self.GetAvatarActorFromActorInfo`) "/Script/ClosedGrounds.CG_WeaponComponent"))
  (`/Engine/EditorBlueprintResources/StandardMacros.IsValid` _returnvalue
    (:`Is Valid`
      (set `self.WeaponComponent` _returnvalue)
      (return))
    (:`Is Not Valid`
      (`self.K2_EndAbility`))))