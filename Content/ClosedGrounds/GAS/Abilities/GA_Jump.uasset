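; GA_Jump is a Gameplay Ability that makes the avatar Character jump and plays a 2D jump sound.
; Activation commits through a local helper that prints a message and ends the ability on failure, then calls Jump and ends immediately without waiting for landing.
; A function that applies GE_Slowdown to the avatar, named for use on landing, exists but is not connected to any event.
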(event `self.K2_ActivateAbility`
  (`parent.K2_ActivateAbility`)
  (bind _returnvalue (`self.K2_CommitAbility`))
  (if _returnvalue
    (bind _ascharacter (cast `Character` (`self.GetAvatarActorFromActorInfo`)))
    (`Character.Jump` _ascharacter)
    (`GameplayStatics.PlaySound2D` "/Game/PlaceholderAssets/Art/Sounds/Chain/Jump/A_JumpV3.A_JumpV3" 1.0 1.0 0.0 null null)
    (`self.K2_EndAbility`)
    (else
      (`KismetSystemLibrary.PrintString` "Ability wasn't commited!")
      (`self.K2_EndAbility`))))

(event `self.K2_OnEndAbility`
  (params (bWasCancelled :type Boolean))
  (if (not bWasCancelled)
    _))

(fn `ApplySlowdownWhenCharacterLand`
  (locals (InASC :type "AbilitySystemComponent Object Reference") (InEffectContext :type "GameplayEffectContextHandle Structure"))
  (bind _output_get (set `local.InASC` (`AbilitySystemBlueprintLibrary.GetAbilitySystemComponent` (`self.GetAvatarActorFromActorInfo`))))
  (set `local.InEffectContext` (`AbilitySystemComponent.MakeEffectContext` _output_get))
  (`AbilitySystemComponent.BP_ApplyGameplayEffectSpecToSelf` (`local.InASC`) (`AbilitySystemComponent.MakeOutgoingSpec` (`local.InASC`) "/Game/ClosedGrounds/GAS/Effects/GE_Slowdown.GE_Slowdown_C" 0.0 (`local.InEffectContext`)))
  (return))