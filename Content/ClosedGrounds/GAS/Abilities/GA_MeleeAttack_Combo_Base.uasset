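; Base melee combo Gameplay Ability that picks its attack montage from ComboMontages by index before running the parent's montage start logic.
; Once a montage starts, it listens for combo window start, window end and combo input gameplay events, then advances the index, wrapping at the array's end.
; Input events record whether they land inside the window; a window closing without timely input resets the index and ends the ability.
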(event `self.OnMontageStart`
  (bind _output_get (set `self.AttackMontage` (`|GetArrayItem` (`self.ComboMontages`) (`self.IndexCounter`))))
  (`/Engine/EditorBlueprintResources/StandardMacros.IsValid` _output_get
    (:`Is Valid`
      (`parent.OnMontageStart`))
    (:`Is Not Valid`
      (`KismetSystemLibrary.PrintString` "There isn't montage!"))))

(event `self.MontageStarted`
  (`AbilityTask_WaitGameplayEvent.WaitGameplayEvent` (struct :`TagName` "GAS.Event.Abilities.Combo.Start") null
    (:`then`
      (`AbilityTask_WaitGameplayEvent.WaitGameplayEvent` (struct :`TagName` "GAS.Event.Abilities.Combo.End") null
        (:`then`
          (`AbilityTask_WaitGameplayEvent.WaitGameplayEvent` (struct :`TagName` "GAS.Event.Abilities.Combo") null
            (:`then`
              (set `self.AttackMontage` (`|GetArrayItem` (`self.ComboMontages`) (`self.IndexCounter`)))
              (if (>= (`self.IndexCounter`) (- (`KismetArrayLibrary.Array_Length` (`self.ComboMontages`)) 1))
                (set `self.IndexCounter` 0)
                (else
                  (`/Engine/EditorBlueprintResources/StandardMacros.IncrementInt` (`self.IndexCounter`)))))
            (:`EventReceived`
              (set `self.IsReceivedInputAtRightTime` (`self.IsWithinComboWindow`)))))
        (:`EventReceived`
          (set `self.IsWithinComboWindow` false)
          (`self.IsReceivedInputAtRightTime`
            (:`then`)
            (:`else`
              (set `self.IndexCounter` 0)
              (`self.K2_EndAbility`))))))
    (:`EventReceived`
      (set `self.IsWithinComboWindow` true)
      (set `self.IsReceivedInputAtRightTime` false))))