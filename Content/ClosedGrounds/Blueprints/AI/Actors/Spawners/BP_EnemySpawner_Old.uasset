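; Enemy spawner actor that places enemies around itself and can send them toward the player.
; On BeginPlay and on each SpawnEnemy call, it spawns one EnemyToSpawn at a random navigable point within its Sphere radius, lifted slightly, and records it in SpawnedEnemies.
; TriggerEnemies calls GoToPlayerEvent on every still-valid spawned enemy.
; A TimeToSpawn timer node is left unconnected, so spawning does not repeat on its own.
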(event `self.ReceiveBeginPlay`
  (bind _randomlocation (`NavigationSystemV1.K2_GetRandomLocationInNavigableRadius` (`self.K2_GetActorLocation`) (`SphereComponent.GetScaledSphereRadius` (`self.Sphere`)) null null :!label _label))
  (bind _returnvalue (`|SpawnActorFromClass` (`self.EnemyToSpawn`) (`KismetMathLibrary.MakeTransform` (+ _randomlocation (0.0 0.0 100.0))) "Undefined" "MultiplyWithRoot" null null))
  (`KismetArrayLibrary.Array_Add` (`self.SpawnedEnemies`) _returnvalue))

(event `SpawnEnemy`
  (goto _label))

(event `TriggerEnemies`
  (for _array_element (`self.SpawnedEnemies`)
    (`/Engine/EditorBlueprintResources/StandardMacros.IsValid` _array_element
      (:`Is Valid`
        (`/Game/ClosedGrounds/Blueprints/Characters/Enemies/BP_EnemyBase.GoToPlayerEvent` _array_element)))))

(fn `UserConstructionScript`)