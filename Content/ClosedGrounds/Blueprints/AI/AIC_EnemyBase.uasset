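; Base AI controller for enemies that starts their behavior tree and sets up targeting when the player is detected.
; On possession it stores the pawn and sets a short timer to defer running the behavior tree held by BP_EnemyBase.
; OnPlayerDetected flags detection in the Blackboard and sets player 0 as attack target.
; It also writes far and close desired distances, queried from the pawn through interface messages.
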(event `self.ReceivePossess`
  (params (PossessedPawn :type "Pawn Object Reference"))
  (set `self.PossessedPawn` PossessedPawn)
  (bind _returnvalue (`KismetSystemLibrary.K2_SetTimerDelegate` (`|CreateDelegate` :!event `HandlePossess`) 0.2))
  (set `self.HandlePossess_TimerHandle` _returnvalue))

(event `HandlePossess`
  (bind _asbp_enemy_base (cast `/Game/ClosedGrounds/Blueprints/Characters/Enemies/BP_EnemyBase` (`self.PossessedPawn`)))
  (bind _behaviortree (`/Game/ClosedGrounds/Blueprints/Characters/Enemies/BP_EnemyBase.BehaviorTree` _asbp_enemy_base)
    (:`then`
      (`self.RunBehaviorTree` _behaviortree))
    (:`else`
      (`KismetSystemLibrary.PrintString` "No Valid Behavior Tree"))))

(event `OnPlayerDetected`
  (bind _returnvalue (`GameplayStatics.GetPlayerCharacter` 0))
  (bind _blackboard (`self.Blackboard`)
    (:`then`
      (bind _output_get (set `self.EnemyBlackboard` _blackboard))
      ; BT waiting for Player Detection
      (`self.DetectsEnemy`)
      ; Set Blackboard Key AttackTarget
      (`BlackboardComponent.SetValueAsObject` _output_get (`self.AttackTargetKeyName`) _returnvalue)
      ; Ssetting Maximal and Minimal distance from AttackTarget
      (`self.SetMaximumDistanceFromAttackTarget`)
      (`self.SetMinimumDistanceFromAttackTarget`)
      (set `self.AttackTarget` _returnvalue))
    (:`else`)))

(fn `DetectsEnemy`
  (`BlackboardComponent.SetValueAsBool` (`self.Blackboard`) (`self.BoolKeyName`) true))

(fn `GetDesiredRangeClose`
  (returns (DesiredDistanceFromTarget :type "Float (double-precision)"))
  (return 0.0))

(fn `GetDesiredRangeFar`
  (returns (DesiredDistanceFromTarget :type "Float (double-precision)"))
  (return 0.0))

(fn `SetMaximumDistanceFromAttackTarget`
  (bind _desireddistancefromtarget (message `/Game/ClosedGrounds/Blueprints/Interfaces/BPI_EnemyAI.GetDesiredRangeFar` (`self.PossessedPawn`)))
  (`BlackboardComponent.SetValueAsFloat` (`self.Blackboard`) (`self.DesiredDistanceFromTarget`) _desireddistancefromtarget))

(fn `SetMinimumDistanceFromAttackTarget`
  (bind _desireddistancefromtarget (message `/Game/ClosedGrounds/Blueprints/Interfaces/BPI_EnemyAI.GetDesiredRangeClose` (`self.PossessedPawn`)))
  (`BlackboardComponent.SetValueAsFloat` (`self.Blackboard`) (`self.DesiredDistanceFromTargeClose`) _desireddistancefromtarget))

(fn `UserConstructionScript`)