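; Base pickup actor that grants a Gameplay Ability System effect to the actor that touches it.
; A timeline started on BeginPlay spins the static mesh around yaw by adding the change in angle each update.
; Sphere overlap fires OnPickUp, which applies the configured GameplayEffect through the overlapping actor's AbilitySystemComponent, plays a sound at the pickup's location and destroys it.
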(event `self.ReceiveBeginPlay`
  (`parent.ReceiveBeginPlay`)
  (bind (_direction _interpolation) (`Timeline|Object_Rotation` :!via `PlayFromStart`)
    (:`Update`
      (bind _output_get (set `self.CurrentStaticMeshRotation` (* _interpolation 360.0)))
      (`SceneComponent.K2_AddRelativeRotation` (`self.StaticMesh`) (`KismetMathLibrary.MakeRotator` 0.0 0.0 (- _output_get (`self.PreviousStaticMeshRotation`))) false false)
      (set `self.Relative Rotation` (`SceneComponent.RelativeRotation` (`self.StaticMesh`)))
      (set `self.PreviousStaticMeshRotation` (`self.CurrentStaticMeshRotation`)))))

(event `self.Sphere.OnComponentBeginOverlap`
  (params (OverlappedComponent :type "PrimitiveComponent Object Reference") (OtherActor :type "Actor Object Reference") (OtherComp :type "PrimitiveComponent Object Reference") (OtherBodyIndex :type Integer) (bFromSweep :type Boolean) (SweepResult :type "HitResult Structure (by ref)"))
  (`self.OnPickUp` OtherActor))

(event `OnPickUp`
  (params (Actor :type "Actor Object Reference"))
  (`self.ApplyGameplayEffect` Actor)
  (`self.PlayPickUpSound`)
  (`self.K2_DestroyActor`))

(fn `ApplyGameplayEffect`
  (params (Actor :type "Actor Object Reference"))
  (bind _returnvalue (`AbilitySystemBlueprintLibrary.GetAbilitySystemComponent` Actor))
  (`AbilitySystemComponent.BP_ApplyGameplayEffectToTarget` :`self` _returnvalue :`GameplayEffectClass` (`self.GameplayEffect`) :`Target` _returnvalue))

(fn `PlayPickUpSound`
  (`GameplayStatics.PlaySoundAtLocation` (`self.Sound`) (`self.K2_GetActorLocation`) (struct) 1.0 1.0 0.0 null null null null))

(fn `UserConstructionScript`)