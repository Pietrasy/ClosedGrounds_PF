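; House spawner actor that serves as the player's day-start point or day-end entrance.
; Spawn enables the house, then either arms it for entry when spawned at day's end or moves the player to its spawn point.
; Interacting inside the box while active notifies the player controller, draws quests, ends the day and saves.
; At day start, leaving DowidzeniaRange plays a stand-up animation, and a timer later hides the house and disables its collision.
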(event `/Game/ClosedGrounds/Blueprints/Interfaces/BPI_Interactable.Interact`
  (params (Interactor :type "Actor Object Reference"))
  (if (`PrimitiveComponent.IsOverlappingActor` (`self.Box`) (`GameplayStatics.GetPlayerCharacter` 0))
    (`self.IsActive`
      (:`then`
        (bind _asbp_player_controller (cast `/Game/ClosedGrounds/Blueprints/Game/BP_PlayerController` (`GameplayStatics.GetPlayerController` 0)))
        (`/Game/ClosedGrounds/Blueprints/Game/BP_PlayerController.HandleHouseEnter` _asbp_player_controller)
        (`self.EnterHouse`))
      (:`else`))))

(event `self.DowidzeniaRange.OnComponentEndOverlap`
  (params (OverlappedComponent :type "PrimitiveComponent Object Reference") (OtherActor :type "Actor Object Reference") (OtherComp :type "PrimitiveComponent Object Reference") (OtherBodyIndex :type Integer))
  (`self.IsStand`
    (:`then`)
    (:`else`
      (`self.CanReact`
        (:`then`
          (`SkeletalMeshComponent.PlayAnimation` (`self.HouseMesh`) "/Game/PlaceholderAssets/Art/Enviroment/Interactables/DabekHouse/Anim/ANIM_DABEK_HOUSEDABEK_HOUSE_RIG_ANIM_DABEKHOUSE_StandUP.ANIM_DABEK_HOUSEDABEK_HOUSE_RIG_ANIM_DABEKHOUSE_StandUP" false)
          (set `self.IsStand` true)
          (`KismetSystemLibrary.K2_SetTimer` null "DisableHouse" 10.0))
        (:`else`)))))

(fn `DisableHouse`
  (`PrimitiveComponent.SetCollisionProfileName` (`self.DowidzeniaRange`) "NoCollision" true)
  (`PrimitiveComponent.SetCollisionProfileName` (`self.Box`) "NoCollision" true)
  (`SceneComponent.SetHiddenInGame` (`self.HouseMesh`) true false)
  (`PrimitiveComponent.SetCollisionProfileName` (`self.HouseMesh`) "NoCollision" true)
  (`PrimitiveComponent.SetCollisionProfileName` (`self.Plane`) "NoCollision" true)
  (`SkeletalMeshComponent.PlayAnimation` (`self.HouseMesh`) "/Game/PlaceholderAssets/Art/Enviroment/Interactables/DabekHouse/Anim/ANIM_DABEK_HOUSEDABEK_HOUSE_RIG_Idle_Start_Pose_002.ANIM_DABEK_HOUSEDABEK_HOUSE_RIG_Idle_Start_Pose_002" false)
  (return))

(fn `EnableHouse`
  (set `self.IsStand` false)
  (`PrimitiveComponent.SetCollisionProfileName` (`self.DowidzeniaRange`) "OnlyInteractWithPlayer" true)
  (`PrimitiveComponent.SetCollisionProfileName` (`self.Box`) "OnlyInteractWithPlayer" true)
  (`SceneComponent.SetHiddenInGame` (`self.HouseMesh`) false false)
  (`PrimitiveComponent.SetCollisionProfileName` (`self.HouseMesh`) "BlockAll" true)
  (`PrimitiveComponent.SetCollisionProfileName` (`self.Plane`) "BlockAll" true)
  (`SkeletalMeshComponent.PlayAnimation` (`self.HouseMesh`) "/Game/PlaceholderAssets/Art/Enviroment/Interactables/DabekHouse/Anim/ANIM_DABEK_HOUSEDABEK_HOUSE_RIG_Idle_Start_Pose_002.ANIM_DABEK_HOUSEDABEK_HOUSE_RIG_Idle_Start_Pose_002" false)
  (return))

(fn `EnterHouse`
  (`CG_QuestManager.DrawQuests` (subsystem `CG_QuestManager`))
  (`CG_DayManager.EndDay` (subsystem `CG_DayManager`))
  (`CG_SaveManager.SaveGame` (subsystem `CG_SaveManager`))
  (set `self.IsActive` false)
  (return))

(fn `Spawn`
  (`parent.Spawn`)
  (`self.EnableHouse`)
  (if (`self.SpawnedOnEndDay`)
    (set `self.IsActive` true)
    (set `self.CanReact` false)
    (return)
    (else
      (set `self.IsActive` false)
      (`self.SpawnPlayer`)
      (set `self.CanReact` true))))

(fn `SpawnPlayer`
  (`self.K2_SetActorLocationAndRotation` (`GameplayStatics.GetPlayerCharacter` 0) (`KismetMathLibrary.TransformLocation` (`self.GetTransform`) (`self.PlayerSpawnPoint`)) (`SceneComponent.RelativeRotation` (`self.Arrow`)) false false)
  (return))

(fn `UserConstructionScript`)