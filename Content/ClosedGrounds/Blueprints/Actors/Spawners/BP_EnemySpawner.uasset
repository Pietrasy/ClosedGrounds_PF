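; Enemy spawner that fills a sphere's navigable area with configured enemies and reacts when an enemy is detected.
; Spawn runs the parent logic, then walks the EnemiesToSpawn class-to-count map, recursively spawning each at random navigable points and storing them in SpawnedEnemies.
; On OnEnemyDetected, it loops that list into SpoconaDupa through a latent Delay, so calls do not fire per element.
; The node setting each enemy's Spawner reference is unconnected.
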(event `self.ReceiveBeginPlay`
  (add `self.OnEnemyDetected` (delegate `OnEnemyDetected_Event`)))

(event `OnEnemyDetected_Event`
  (for _array_element (`self.SpawnedEnemies`)
    (`KismetSystemLibrary.Delay` 0.001)
    (`/Game/ClosedGrounds/Blueprints/Characters/Enemies/BP_EnemyBase.SpoconaDupa` _array_element)))

(fn `ChooseEnemyToSpawn`
  (bind _keys (`BlueprintMapLibrary.Map_Keys` (`self.EnemiesToSpawn`)))
  (for (_array_element _array_index) _keys
    (set `self.EnemyToSpawn` _array_element)
    (bind _values (`BlueprintMapLibrary.Map_Values` (`self.EnemiesToSpawn`)))
    (set `self.EnemyCounter` (`|GetArrayItem` _values _array_index))
    (`self.CountSpawnedEnemies`))
  (return))

(fn `CountSpawnedEnemies`
  (if (> (`self.EnemyCounter`) 0)
    (`/Engine/EditorBlueprintResources/StandardMacros.DecrementInt` (`self.EnemyCounter`)
      (:`  `
        (bind _randomlocation (`NavigationSystemV1.K2_GetRandomLocationInNavigableRadius` (`self.K2_GetActorLocation`) (`SphereComponent.GetScaledSphereRadius` (`self.Sphere`)) null null))
        (bind _returnvalue (`|SpawnActorFromClass` (`self.EnemyToSpawn`) (`KismetMathLibrary.MakeTransform` (+ _randomlocation (0.0 0.0 100.0))) "Undefined" "MultiplyWithRoot" null null))
        (`KismetArrayLibrary.Array_Add` (`self.SpawnedEnemies`) _returnvalue)
        (`self.CountSpawnedEnemies`)))
    (else
      (return))))

(fn `Spawn`
  (`parent.Spawn`)
  (`self.ChooseEnemyToSpawn`))

(fn `UserConstructionScript`)