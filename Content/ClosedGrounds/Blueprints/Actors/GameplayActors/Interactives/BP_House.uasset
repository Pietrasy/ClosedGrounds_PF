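; BP_House is an interactive gameplay actor for a house that can place the player at its own spawn point.
; Its Activate event runs the parent logic, then enables the gameplay actor.
; SpawnPlayer moves the existing first player character to the PlayerSpawnPoint location and rotation at unit scale, rather than creating a new pawn.
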(event `self.Activate`
  (`parent.Activate`)
  (`self.EnableGameplayActor`))

(fn `SpawnPlayer`
  (`self.K2_SetActorTransform` (`GameplayStatics.GetPlayerCharacter` 0) (`KismetMathLibrary.MakeTransform` (.location (`SceneComponent.K2_GetComponentToWorld` (`self.PlayerSpawnPoint`))) (.rotation (`SceneComponent.K2_GetComponentToWorld` (`self.PlayerSpawnPoint`)))) false false)
  (return))

(fn `UserConstructionScript`
  (`parent.UserConstructionScript`))