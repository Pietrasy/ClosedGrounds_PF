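; Interactive gameplay actor with a static mesh that plays a 2D sound when interacted with.
; On BeginPlay it runs the parent logic, then enables or disables itself based on a validity check of IsPersistent.
; Enabling shows the mesh with query and physics collision, while disabling hides it in game and turns collision off.
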(event `self.ReceiveBeginPlay`
  (`parent.ReceiveBeginPlay`)
  (`self.bIsPersistent`
    (:`then`
      (`self.EnableGameplayActor`))
    (:`else`
      (`self.DisableGameplayActor`))))

(event `/Game/ClosedGrounds/Blueprints/Interfaces/BPI_Interactable.Interact`
  (params (Interactor :type "Actor Object Reference"))
  (`GameplayStatics.PlaySound2D` (`self.InteractionSound`) 1.0 1.0 0.0 null null))

(fn `DisableGameplayActor`
  (`SceneComponent.SetHiddenInGame` (`self.StaticMeshComponent`) true false)
  (`PrimitiveComponent.SetCollisionEnabled` (`self.StaticMeshComponent`) "NoCollision")
  (return))

(fn `EnableGameplayActor`
  (`SceneComponent.SetHiddenInGame` (`self.StaticMeshComponent`) false false)
  (`PrimitiveComponent.SetCollisionEnabled` (`self.StaticMeshComponent`) "QueryAndPhysics")
  (return))

(fn `UserConstructionScript`)