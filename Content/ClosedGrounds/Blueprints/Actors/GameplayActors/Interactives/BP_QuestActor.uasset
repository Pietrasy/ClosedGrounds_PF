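; BP_QuestActor is an interactive gameplay actor that advances a quest objective when the player interacts with it.
; On activation it becomes interactable and enabled only if its objective tag matches, non-exactly, any of today's quest tags from the quest manager.
; On interaction, when interactable, it reports that tag to the quest manager, then disables itself unless marked persistent.
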(event `/Game/ClosedGrounds/Blueprints/Interfaces/BPI_Interactable.Interact`
  (params (Interactor :type "Actor Object Reference"))
  (`parent.Interact` Interactor)
  (`self.bIsInteractable`
    (:`then`
      (`CG_QuestManager.UpdateObjective` (subsystem `CG_QuestManager`) (`self.ObjectiveTag`))
      (if (not (`self.bIsPersistent`))
        (`self.DisableGameplayActor`)))
    (:`else`)))

(event `self.Activate`
  (`parent.Activate`)
  (if (`self.CheckQuestsTagsMatching`)
    (set `self.bIsInteractable` true)
    (`self.EnableGameplayActor`)))

(fn `CheckQuestsTagsMatching`
  (returns (bIsMatch :type Boolean))
  (bind _returnvalue (`CG_QuestManager.GetTodayQuestsTags` (subsystem `CG_QuestManager`)))
  (return (`BlueprintGameplayTagLibrary.MatchesAnyTags` (`self.ObjectiveTag`) _returnvalue)))

(fn `UserConstructionScript`
  (`parent.UserConstructionScript`))