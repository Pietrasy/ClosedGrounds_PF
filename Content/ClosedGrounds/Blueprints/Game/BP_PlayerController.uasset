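; Player controller that routes Enhanced Input to movement and look, and triggers melee, jump and dash as GAS abilities by tag.
; InitUI builds a layered root widget with HUD and quest panel.
; Pause and dev-only shop toggles lazily create widgets and switch game pause, cursor and input mode.
; Handlers hide the layers for the death screen or house shop; leaving the house restores them and starts the GameMode countdown.
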(event `EnhancedInput|/Game/ClosedGrounds/Inputs/InputActions/IA_Move`
  (params (ActionValue :type "Vector2D Structure") (ElapsedSeconds :type "Float (double-precision)") (TriggeredSeconds :type "Float (double-precision)") (InputAction :type "InputAction Object Reference" :default "/Game/ClosedGrounds/Inputs/InputActions/IA_Move.IA_Move"))
  ; Move and look around
  (:`Triggered`
    (`Pawn.AddMovementInput` (`self.PlayerCharacter`) (`self.GetActorRightVector` (`self.PlayerCharacter`)) ActionValue_X false)
    (`Pawn.AddMovementInput` (`self.PlayerCharacter`) (`self.GetActorForwardVector` (`self.PlayerCharacter`)) ActionValue_Y false)))

(event `EnhancedInput|/Game/ClosedGrounds/Inputs/InputActions/IA_Look`
  (params (ActionValue :type "Vector2D Structure") (ElapsedSeconds :type "Float (double-precision)") (TriggeredSeconds :type "Float (double-precision)") (InputAction :type "InputAction Object Reference" :default "/Game/ClosedGrounds/Inputs/InputActions/IA_Look.IA_Look"))
  ; Move and look around
  (:`Triggered`
    (`self.AddYawInput` ActionValue_X)
    (`self.AddPitchInput` ActionValue_Y)))

(event `EnhancedInput|/Game/ClosedGrounds/Inputs/InputActions/IA_Attack`
  (params (ActionValue :type Boolean) (ElapsedSeconds :type "Float (double-precision)") (TriggeredSeconds :type "Float (double-precision)") (InputAction :type "InputAction Object Reference" :default "/Game/ClosedGrounds/Inputs/InputActions/IA_Attack.IA_Attack"))
  (:`Started`
    (`AbilitySystemComponent.TryActivateAbilitiesByTag` (`AbilitySystemBlueprintLibrary.GetAbilitySystemComponent` (`self.PlayerCharacter`)) (`BlueprintGameplayTagLibrary.MakeLiteralGameplayTagContainer` (struct :`GameplayTags` (struct :`(TagName` "GAS.Ability.MeleeAttack")))) true)))

(event `EnhancedInput|/Game/ClosedGrounds/Inputs/InputActions/IA_Jump`
  (params (ActionValue :type Boolean) (ElapsedSeconds :type "Float (double-precision)") (TriggeredSeconds :type "Float (double-precision)") (InputAction :type "InputAction Object Reference" :default "/Game/ClosedGrounds/Inputs/InputActions/IA_Jump.IA_Jump"))
  (:`Started`
    (`AbilitySystemComponent.TryActivateAbilitiesByTag` (`AbilitySystemBlueprintLibrary.GetAbilitySystemComponent` (`self.PlayerCharacter`)) (`BlueprintGameplayTagLibrary.MakeLiteralGameplayTagContainer` (struct :`GameplayTags` (struct :`(TagName` "GAS.Ability.Jump")))) true)))

(event `EnhancedInput|/Game/ClosedGrounds/Inputs/InputActions/IA_Dash`
  (params (ActionValue :type Boolean) (ElapsedSeconds :type "Float (double-precision)") (TriggeredSeconds :type "Float (double-precision)") (InputAction :type "InputAction Object Reference" :default "/Game/ClosedGrounds/Inputs/InputActions/IA_Dash.IA_Dash"))
  (:`Started`
    (`AbilitySystemComponent.TryActivateAbilitiesByTag` (`AbilitySystemBlueprintLibrary.GetAbilitySystemComponent` (`self.PlayerCharacter`)) (`BlueprintGameplayTagLibrary.MakeLiteralGameplayTagContainer` (struct :`GameplayTags` (struct :`(TagName` "GAS.Ability.Dash")))) true)))

(event `EnhancedInput|/Game/ClosedGrounds/Inputs/InputActions/IA_Pause`
  (params (ActionValue :type Boolean) (ElapsedSeconds :type "Float (double-precision)") (TriggeredSeconds :type "Float (double-precision)") (InputAction :type "InputAction Object Reference" :default "/Game/ClosedGrounds/Inputs/InputActions/IA_Pause.IA_Pause"))
  ; Pause Game
  (:`Started`
    (`/Engine/EditorBlueprintResources/StandardMacros.IsValid` (`self.PauseRef`)
      (:`Is Valid`
        (if (`GameplayStatics.IsGamePaused`)
          (`self.HidePauseMenu`)
          (else
            (`self.DisplayPauseMenu`))))
      (:`Is Not Valid`
        (bind _returnvalue (`|CreateWidget` "/Game/ClosedGrounds/Blueprints/Widgets/Menus/WBP_Pause.WBP_Pause_C"))
        (set `self.PauseRef` _returnvalue)
        (`self.DisplayPauseMenu`)))))

(event `EnhancedInput|/Game/ClosedGrounds/Inputs/InputActions/IA_Shop`
  (params (ActionValue :type Boolean) (ElapsedSeconds :type "Float (double-precision)") (TriggeredSeconds :type "Float (double-precision)") (InputAction :type "InputAction Object Reference" :default "/Game/ClosedGrounds/Inputs/InputActions/IA_Shop.IA_Shop"))
  ; Shop (Dev only)
  (:`Started`
    (`/Engine/EditorBlueprintResources/StandardMacros.IsValid` (`self.ShopRef`)
      (:`Is Valid`
        (if (`GameplayStatics.IsGamePaused`)
          (`self.HideShop`)
          (else
            (`self.DisplayShop`))))
      (:`Is Not Valid`
        (bind _returnvalue (`|CreateWidget` "/Game/ClosedGrounds/Blueprints/Widgets/Shop/WBP_Layer_Shop.WBP_Layer_Shop_C"))
        (set `self.ShopRef` _returnvalue)
        (`self.DisplayShop`)))))

(event `self.InitUI`
  (`parent.InitUI`)
  (bind _returnvalue (`|CreateWidget` "/Game/ClosedGrounds/Blueprints/Widgets/WBP_Root.WBP_Root_C"))
  (bind _output_get (set `self.RootWidget` _returnvalue))
  (`CG_WidgetBase.SetWidgetController` _output_get (`self.WidgetController`))
  (bind _returnvalue_2 (`|CreateWidget` "/Game/ClosedGrounds/Blueprints/Widgets/WBP_Layer_HUD.WBP_Layer_HUD_C"))
  (`/Game/ClosedGrounds/Blueprints/Widgets/WBP_Root.AddToLayer` :`self` (`self.RootWidget`) :`InWidget` _returnvalue_2 :`Size To Content` true)
  (bind _returnvalue_3 (`|CreateWidget` "/Game/ClosedGrounds/Blueprints/Widgets/Quests/WBP_QuestPanel.WBP_QuestPanel_C"))
  (`/Game/ClosedGrounds/Blueprints/Widgets/WBP_Root.AddToLayer` (`self.RootWidget`) _returnvalue_3 (make `Anchors` (1.0 0.0) (1.0 0.0)) (`KismetMathLibrary.MakeVector2D` 1.0) true)
  (`UserWidget.AddToViewport` (`self.RootWidget`) 0))

(fn `DisplayPauseMenu`
  (`UserWidget.AddToViewport` (`self.PauseRef`) 0)
  (`GameplayStatics.SetGamePaused` true)
  (set `PlayerController.bShowMouseCursor` true (`GameplayStatics.GetPlayerController` 0))
  (`WidgetBlueprintLibrary.SetInputMode_GameAndUIEx` (`GameplayStatics.GetPlayerController` 0) (`self.PauseRef`)))

(fn `DisplayShop`
  (`GameplayStatics.SetGamePaused` true)
  (set `PlayerController.bShowMouseCursor` true (`GameplayStatics.GetPlayerController` 0))
  (`WidgetBlueprintLibrary.SetInputMode_GameAndUIEx` (`GameplayStatics.GetPlayerController` 0) (`self.ShopRef`)))

(fn `HandleHouseEnter`
  (`/Game/ClosedGrounds/Blueprints/Widgets/WBP_Root.HideAllLayers` (`self.RootWidget`))
  (bind _returnvalue (`|CreateWidget` "/Game/ClosedGrounds/Blueprints/Widgets/Shop/WBP_Layer_Shop.WBP_Layer_Shop_C"))
  (bind _output_get (set `self.Shop` _returnvalue))
  (`UserWidget.AddToViewport` _output_get 0)
  (`self.DisplayShop`))

(fn `HandleHouseExit`
  (`/Game/ClosedGrounds/Blueprints/Widgets/WBP_Root.ShowAllLayers` (`self.RootWidget`))
  (bind _asbp_game_mode (cast `/Game/ClosedGrounds/Blueprints/Game/BP_GameMode` (`GameplayStatics.GetGameMode`)))
  (`/Game/ClosedGrounds/Blueprints/Game/BP_GameMode.StartCountdown` _asbp_game_mode))

(fn `HandlePlayerDeath`
  (`/Game/ClosedGrounds/Blueprints/Widgets/WBP_Root.HideAllLayers` (`self.RootWidget`))
  (bind _returnvalue (`|CreateWidget` "/Game/ClosedGrounds/Blueprints/Widgets/Menus/WBP_DeathScreen.WBP_DeathScreen_C"))
  (`UserWidget.AddToViewport` _returnvalue 0)
  (`WidgetBlueprintLibrary.SetInputMode_GameAndUIEx` (`GameplayStatics.GetPlayerController` 0) _returnvalue "LockAlways")
  (set `PlayerController.bShowMouseCursor` true (`GameplayStatics.GetPlayerController` 0)))

(fn `HidePauseMenu`
  (`Widget.RemoveFromParent` (`self.PauseRef`))
  (`GameplayStatics.SetGamePaused` false)
  (set `PlayerController.bShowMouseCursor` false (`GameplayStatics.GetPlayerController` 0))
  (`WidgetBlueprintLibrary.SetInputMode_GameOnly` (`GameplayStatics.GetPlayerController` 0)))

(fn `HideShop`
  (`Widget.RemoveFromParent` (`self.ShopRef`))
  (`GameplayStatics.SetGamePaused` false)
  (set `PlayerController.bShowMouseCursor` false (`GameplayStatics.GetPlayerController` 0))
  (`WidgetBlueprintLibrary.SetInputMode_GameOnly` (`GameplayStatics.GetPlayerController` 0)))

(fn `LookInterpolationRelativeToXAxis`
  (params (ValueX :type "Float (double-precision)") (InterpSpeed :type "Float (double-precision)" :default 90.0))
  (locals (InputAxisLookX :type "Float (double-precision)"))
  (bind _output_get (set `local.InputAxisLookX` (`KismetMathLibrary.FInterpTo` (`local.InputAxisLookX`) (`local.ValueX`) (`GameplayStatics.GetWorldDeltaSeconds`) 120.0)))
  (`self.AddYawInput` _output_get)
  (return))

(fn `LookInterpolationRelativeToYAxis`
  (params (ValueY :type "Float (double-precision)") (InterpSpeed :type "Float (double-precision)" :default 90.0))
  (locals (InputAxisLookY :type "Float (double-precision)"))
  (bind _output_get (set `local.InputAxisLookY` (`KismetMathLibrary.FInterpTo` (`local.InputAxisLookY`) (`local.ValueY`) (`GameplayStatics.GetWorldDeltaSeconds`) (`local.InterpSpeed`))))
  (`self.AddPitchInput` _output_get)
  (return))

(fn `UserConstructionScript`)