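; Game mode that sets the day's cloud material, toggles recording over the play session and forwards player death to the character's restart.
; Tick holds a fog countdown that broadcasts a value interpolated over the day, then kills the player with a GAS damage effect when time expires.
; The countdown start and the bindings for fog reset and quest-completion sound sit in unconnected nodes.
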(event `self.StartGame`
  (`parent.StartGame`)
  (bind _outactors (`GameplayStatics.GetAllActorsWithTag` "Cloud"))
  (bind _asvolumetric_cloud (cast `VolumetricCloud` (`|GetArrayItem` _outactors)))
  (`VolumetricCloudComponent.SetMaterial` (`VolumetricCloud.VolumetricCloudComponent` _asvolumetric_cloud) (`CG_DayManagerComponent.GetTodayVolumetricCloudMaterial` (`self.DayManagerComponent`))))

(event `self.ReceiveTick`
  (params (DeltaSeconds :type "Float (single-precision)"))
  (bind _returnvalue (`AbilitySystemBlueprintLibrary.GetAbilitySystemComponent` (`GameplayStatics.GetPlayerCharacter` 0)))
  (`self.IsCounting`
    (:`then`
      (set `self.ElapsedTime` (+ (`self.ElapsedTime`) (`GameplayStatics.GetWorldDeltaSeconds`)))
      (set `self.Alpha` (`KismetMathLibrary.FClamp` (`KismetMathLibrary.SafeDivide` (`self.ElapsedTime`) (`self.DayDuration`))))
      (set `self.CurrentFogValue` (`KismetMathLibrary.Lerp` (`self.StartFogValue`) (`self.FogTreshold`) (`self.Alpha`)))
      (if (>= (`self.Alpha`) 1.0)
        (set `self.IsCounting` false)
        ; Kill player
        (bind _returnvalue_2 (`AbilitySystemBlueprintLibrary.AssignTagSetByCallerMagnitude` (`AbilitySystemComponent.MakeOutgoingSpec` _returnvalue "/Game/ClosedGrounds/GAS/Effects/GE_Damage_Instant.GE_Damage_Instant_C" 0.0 (`AbilitySystemComponent.MakeEffectContext` _returnvalue)) (struct :`TagName` "GAS.Data.Damage") 1000.0))
        (`AbilitySystemComponent.BP_ApplyGameplayEffectSpecToSelf` _returnvalue _returnvalue_2)
        (else
          (`self.OnFogUpdate` (`self.CurrentFogValue`)))))
    (:`else`)))

(event `self.ReceiveBeginPlay`
  (`parent.ReceiveBeginPlay`)
  (`VisualLoggerKismetLibrary.EnableRecording` true))

(event `self.ReceiveEndPlay`
  (params (EndPlayReason :type "EEndPlayReason Enum" :default "Destroyed"))
  (`parent.ReceiveEndPlay` EndPlayReason)
  (`VisualLoggerKismetLibrary.EnableRecording` false))

(event `OnDayEnded_Event`
  (`self.ResetFog`))

(event `OnFinishedAllQuests_Event`
  (`GameplayStatics.PlaySound2D` "/Game/PlaceholderAssets/A_CWLmuwi.A_CWLmuwi" 1.0 1.0 0.0 null null))

(event `self.HandlePlayerDeath`
  (bind _asbp_player_character (cast `/Game/ClosedGrounds/Blueprints/Characters/Player/BP_PlayerCharacter` (`GameplayStatics.GetPlayerCharacter` 0)))
  (`/Game/ClosedGrounds/Blueprints/Characters/Player/BP_PlayerCharacter.OnRestartGame` _asbp_player_character))

(fn `ResetFog`
  (set `self.IsCounting` false)
  (set `self.CurrentFogValue` 0.0)
  (return))

(fn `StartCountdown`
  (set `self.IsCounting` true)
  (return))

(fn `UserConstructionScript`)