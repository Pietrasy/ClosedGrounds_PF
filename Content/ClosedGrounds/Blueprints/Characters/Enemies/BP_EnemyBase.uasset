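; Base enemy character that detects the player, performs melee attacks through the Gameplay Ability System and handles its death.
; PlayerDetection overlap fires once to notify AIC_EnemyBase, and BeginPlay also binds an event to trigger-box entry.
; Attack activates abilities by the MeleeAttack tag, while death detaches the controller and disables capsule collision.
; Getters supply close and far desired ranges; several stub events and disconnected blackboard attack-state nodes remain unused.
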(event `self.PlayerDetection.OnComponentBeginOverlap`
  (params (OverlappedComponent :type "PrimitiveComponent Object Reference") (OtherActor :type "Actor Object Reference") (OtherComp :type "PrimitiveComponent Object Reference") (OtherBodyIndex :type Integer) (bFromSweep :type Boolean) (SweepResult :type "HitResult Structure (by ref)"))
  (`/Engine/EditorBlueprintResources/StandardMacros.DoOnce` false
    (:`Completed`
      (`self.SpoconaDupa`))))

(event `SpoconaDupa`
  (`/Engine/EditorBlueprintResources/StandardMacros.DoOnce` false
    (:`Completed`
      (bind _asaic_enemy_base (cast `/Game/ClosedGrounds/Blueprints/AI/AIC_EnemyBase` (`self.GetController`)))
      (`/Game/ClosedGrounds/Blueprints/AI/AIC_EnemyBase.OnPlayerDetected` _asaic_enemy_base))))

(event `GoToPlayerEvent`)

(event `/Game/ClosedGrounds/Blueprints/Interfaces/BPI_EnemyAI.GoToPlayer`)

(event `self.ReceiveBeginPlay`
  (`parent.ReceiveBeginPlay`)
  (add `self.OnTriggerBoxEnter` (`|CreateDelegate` :!event `GoToPlayerEvent`)))

(event `/Game/ClosedGrounds/Blueprints/Interfaces/BPI_EnemyAI.Attack`
  (`AbilitySystemComponent.TryActivateAbilitiesByTag` (`self.AbilitySystemComponent`) (`BlueprintGameplayTagLibrary.MakeLiteralGameplayTagContainer` (struct :`GameplayTags` (struct :`(TagName` "GAS.Ability.MeleeAttack")))) true))

(event `self.HandleDeath`
  (`parent.HandleDeath`)
  (`self.DetachFromControllerPendingDestroy`)
  (`PrimitiveComponent.SetCollisionEnabled` (`self.CapsuleComponent`) "NoCollision"))

(event `CheckState`
  ; Check if enemy is attacking for condition check in BT_Spitter (Currently dead code, but do not delete)
)

(fn `GetDesiredRangeClose`
  (returns (DesiredDistanceFromTarget :type "Float (double-precision)"))
  (return 0.0))

(fn `GetDesiredRangeFar`
  (returns (DesiredDistanceFromTarget :type "Float (double-precision)"))
  (return 950.0))

(fn `UserConstructionScript`)