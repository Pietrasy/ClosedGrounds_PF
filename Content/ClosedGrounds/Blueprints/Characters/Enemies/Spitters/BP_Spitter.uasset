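; BP_Spitter is a ranged enemy character that attacks by spawning nut projectiles.
; Its Attack event runs the parent attack, then sets a timer, apparently to delay the projectile spawn.
; SpawnNutProjectile always spawns the configured projectile class at ProjectileSpawnPoint, with the spitter as owner and instigator.
; Getter functions expose its close and far desired combat ranges.
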(event `/Game/ClosedGrounds/Blueprints/Interfaces/BPI_EnemyAI.Attack`
  (`parent.Attack`)
  (`KismetSystemLibrary.K2_SetTimerDelegate` (`|CreateDelegate` :!event `SpawnProjectile`) (`self.Time`)))

(event `SpawnProjectile`
  (`self.SpawnNutProjectile`))

(fn `GetDesiredRangeClose`
  (returns (DesiredDistanceFromTarget :type "Float (double-precision)"))
  (return (`self.DesiredRangeClose`)))

(fn `GetDesiredRangeFar`
  (returns (DesiredDistanceFromTarget :type "Float (double-precision)"))
  (return (`self.DesiredRangeFar`)))

(fn `SpawnNutProjectile`
  (`|SpawnActorFromClass` (`self.ProjectileClass`) (`SceneComponent.K2_GetComponentToWorld` (`self.ProjectileSpawnPoint`)) "AlwaysSpawn" "MultiplyWithRoot" self self)
  (return))

(fn `UserConstructionScript`
  (`parent.UserConstructionScript`))