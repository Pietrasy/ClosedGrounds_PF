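; Player character Blueprint that handles death and restart with screen fades and input toggling.
; Tick feeds its location to a material parameter collection for grass trampling and syncs a GAS falling tag with movement.
; WaitForEvents registers gameplay-event listeners: Slowdown, Champion and timed Hype scale walk speed, Stun briefly blocks movement, and Honey Rush, Hunger and Burn only print.
; Fog post-process setup is disconnected, leaving only its parameter update event.
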(event `self.ReceiveTick`
  (params (DeltaSeconds :type "Float (single-precision)"))
  (`self.SetGrassTramplingPosition`)
  (`self.CheckingIfCharacterFalling`))

(event `self.HandleDeath`
  (bind _returnvalue (`GameplayStatics.GetPlayerController` 0))
  (`parent.HandleDeath`)
  (`/Engine/EditorBlueprintResources/StandardMacros.IsValid` (`GameplayStatics.GetPlayerController` 0)
    (:`Is Valid`
      (`self.DisableInput` _returnvalue _returnvalue)
      (`PlayerCameraManager.StartCameraFade` (`GameplayStatics.GetPlayerCameraManager` 0) 0.0 1.0 1.0 (struct :`A` 1.0) false true)
      (bind _asbp_player_controller (cast `/Game/ClosedGrounds/Blueprints/Game/BP_PlayerController` (`GameplayStatics.GetPlayerController` 0)))
      (`/Game/ClosedGrounds/Blueprints/Game/BP_PlayerController.HandlePlayerDeath` _asbp_player_controller))))

(event `OnRestartGame`
  (bind _returnvalue (`GameplayStatics.GetPlayerController` 0))
  (`self.EnableInput` _returnvalue _returnvalue)
  (`PlayerCameraManager.StartCameraFade` (`GameplayStatics.GetPlayerCameraManager` 0) 1.0 0.0 1.0 (struct :`A` 1.0) false true)
  (`self.HandleSpawn`))

(event `self.ReceiveBeginPlay`
  (`parent.ReceiveBeginPlay`))

(event `UpdateFogParameter`
  (params (FogValue :type "Float (double-precision)"))
  (`MaterialInstanceDynamic.SetScalarParameterValue` (`self.FogInstance`) "Fog Distance" FogValue))

(event `WaitForEvents`
  (`AbilityAsync_WaitGameplayEvent.WaitGameplayEventToActor` null (struct :`TagName` "GAS.Effect.HoneyRush")
    (:`then`
      (`AbilityAsync_WaitGameplayEvent.WaitGameplayEventToActor` null (struct :`TagName` "GAS.Effect.Slowdown")
        (:`then`
          (`AbilityAsync_WaitGameplayEvent.WaitGameplayEventToActor` null (struct :`TagName` "GAS.Effect.Hunger")
            (:`then`
              (`AbilityAsync_WaitGameplayEvent.WaitGameplayEventToActor` null (struct :`TagName` "GAS.State.Stunned")
                (:`then`
                  (`AbilityAsync_WaitGameplayEvent.WaitGameplayEventToActor` null (struct :`TagName` "GAS.State.Champion")
                    (:`then`
                      (`AbilityAsync_WaitGameplayEvent.WaitGameplayEventToActor` null (struct :`TagName` "GAS.Effect.Hype")
                        (:`then`
                          (`AbilityAsync_WaitGameplayEvent.WaitGameplayEventToActor` null (struct :`TagName` "GAS.Effect.Burn")
                            (:`EventReceived`
                              (`KismetSystemLibrary.PrintString` "Fire Applied!"))))
                        (:`EventReceived`
                          ; Hyped Effect activating/deactivating
                          (set `CharacterMovementComponent.MaxWalkSpeed` (* (`CharacterMovementComponent.MaxWalkSpeed` (`self.CharacterMovement`)) (`self.HypedMovementBuff`)) (`self.CharacterMovement`))
                          (`KismetSystemLibrary.K2_SetTimerDelegate` (`|CreateDelegate` :!event `OnHypedEnd`) 1.2))))
                    (:`EventReceived`
                      (`self.ApplyChampion`))))
                (:`EventReceived`
                  ; Disabling/Enabling movement on Stun
                  (message `/Game/ClosedGrounds/Blueprints/Interfaces/BPI_PlayerController.ToggleMovement` (`GameplayStatics.GetPlayerController` 0) false)
                  (`KismetSystemLibrary.K2_SetTimerDelegate` (`|CreateDelegate` :!event `OnStunEnd`) 0.5))))
            (:`EventReceived`
              (`KismetSystemLibrary.PrintString` "Hunger Applied!"))))
        (:`EventReceived`
          (`self.SlowdownEffect`))))
    (:`EventReceived`
      (`KismetSystemLibrary.PrintString` "Honey Rush Applied!"))))

(event `OnStunEnd`
  ; Disabling/Enabling movement on Stun
  (message `/Game/ClosedGrounds/Blueprints/Interfaces/BPI_PlayerController.ToggleMovement` (`GameplayStatics.GetPlayerController` 0) true))

(event `OnHypedEnd`
  ; Hyped Effect activating/deactivating
  (set `CharacterMovementComponent.MaxWalkSpeed` (`self.DefultMaxWalkSpeed`) (`self.CharacterMovement`)))

(fn `ApplyChampion`
  (locals (ChampionMovementDebuf :type "Float (double-precision)" :default 0.5))
  ; Chamption
  (set `CharacterMovementComponent.MaxWalkSpeed` (* (`CharacterMovementComponent.MaxWalkSpeed` (`self.CharacterMovement`)) (`local.ChampionMovementDebuf`)) (`self.CharacterMovement`)))

(fn `CheckingIfCharacterFalling`
  (if (`NavMovementComponent.IsFalling` (`self.CharacterMovement`))
    (if (not (`GameplayTagAssetInterface.HasMatchingGameplayTag` (`AbilitySystemBlueprintLibrary.GetAbilitySystemComponent` null) (struct :`TagName` "GAS.State.Falling")))
      (`AbilitySystemComponent.BP_ApplyGameplayEffectToSelf` :`self` (`AbilitySystemBlueprintLibrary.GetAbilitySystemComponent` null) :`GameplayEffectClass` "/Game/ClosedGrounds/GAS/Effects/GE_Falling.GE_Falling_C")
      (return))
    (else
      (`AbilitySystemComponent.RemoveActiveEffectsWithGrantedTags` (`AbilitySystemBlueprintLibrary.GetAbilitySystemComponent` null) (struct :`GameplayTags` (struct :`(TagName` "GAS.State.Falling"))))
      (return))))

(fn `GetHandSwayData`
  (returns (InSidewaysMove :type "Float (double-precision)") (InForwardMove :type "Float (double-precision)"))
  (bind (_returnvalue_x _returnvalue_y) (`KismetMathLibrary.BreakVector2D` (`|GetInputActionValue`)))
  (return _returnvalue_x _returnvalue_y))

(fn `SetGrassTramplingPosition`
  (`KismetMaterialLibrary.SetVectorParameterValue` "/Game/PlaceholderAssets/Art/Enviroment/Nature/Grass/MPC_PlayerPosition.MPC_PlayerPosition" "PlayerPosition" (`KismetMathLibrary.Conv_VectorToLinearColor` (`self.K2_GetActorLocation`)))
  (return))

(fn `SlowdownEffect`
  (locals (SlowdownDebuff :type "Float (double-precision)" :default 0.75))
  ; Slowing down Player
  (set `CharacterMovementComponent.MaxWalkSpeed` (* (`CharacterMovementComponent.MaxWalkSpeed` (`self.CharacterMovement`)) (`local.SlowdownDebuff`)) (`self.CharacterMovement`)))

(fn `UserConstructionScript`)